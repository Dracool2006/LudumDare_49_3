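; BP_FieldPoint is a single field cell that stores a structure type and whether it is passable.
; SetStruct switches on the type ID to set the static mesh and passable flag, defaulting to a blocked cell on BeginPlay; GetStruct returns both values.
; SetAnimTextura picks a material by attack index and sub-index, including rocket and meteorite, creates dynamic instances once, then assigns the chosen material to the mesh slots.
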(event Custom|SetStruct
  (params (iIndex :type Integer))
  (bind _staticmesh (Variables|Default|GetStaticMesh))
  (bind _output_get (Variables|Default|SetiIdStruct iIndex))
  (switch int _output_get
    (:0
      (Components|StaticMesh|SetStaticMesh _staticmesh "/Game/LD49_Game_Folder/Assets/Areas/AreaBlock12.AreaBlock12")
      (Variables|Default|SetbPassable false))
    (:1
      (Components|StaticMesh|SetStaticMesh _staticmesh "/Game/LD49_Game_Folder/Assets/Areas/AreaMove11.AreaMove11")
      (Variables|Default|SetbPassable true))
    (:2
      (Components|StaticMesh|SetStaticMesh _staticmesh "/Game/LD49_Game_Folder/Assets/Areas/AreaBlock2.AreaBlock2")
      (Variables|Default|SetbPassable false))
    (:3
      (Components|StaticMesh|SetStaticMesh _staticmesh "/Game/LD49_Game_Folder/Assets/Areas/AreaBlock6.AreaBlock6")
      (Variables|Default|SetbPassable false))
    (:4
      (Components|StaticMesh|SetStaticMesh _staticmesh 0)
      (Variables|Default|SetbPassable true))
    (:5
      (Components|StaticMesh|SetStaticMesh _staticmesh 0)
      (Variables|Default|SetbPassable true))
    (:6
      (Components|StaticMesh|SetStaticMesh _staticmesh 0)
      (Variables|Default|SetbPassable true))
    (:7
      (Components|StaticMesh|SetStaticMesh _staticmesh 0)
      (Variables|Default|SetbPassable false))
    (:8
      (Components|StaticMesh|SetStaticMesh _staticmesh 0)
      (Variables|Default|SetbPassable false))
    (:9
      (Components|StaticMesh|SetStaticMesh _staticmesh 0)
      (Variables|Default|SetbPassable false))))

(event Custom|SetAnimTextura
  (params (iIndex :type Integer) (iSubIndex :type Integer))
  (bind _returnvalue (+ iSubIndex 1))
  (bind _returnvalue_2 (Math|Integer|Absolute(Integer) _returnvalue))
  (switch int (- iIndex 1)
    (:Default
      (switch int _returnvalue_2 :!label _label
        (:Default
          ;[1 1 1] Материалы первых двух атак
          (Variables|Default|SetMaterial "/Engine/MapTemplates/Materials/BasicAsset01.BasicAsset01" :!label _label_2))
        (:0
          (goto _label_2))
        (:1
          (Variables|Default|SetMaterial "/Game/LD49_Game_Folder/Assets/PeopleGroups/BlueGroup/Band.Band"))))
    (:0
      (goto _label))
    (:1
      (switch int _returnvalue_2
        (:Default
          ;[1 1 1] Ракета
          (Variables|Default|SetMaterial "/Engine/EngineMaterials/BaseFlattenMaterial.BaseFlattenMaterial" :!label _label_3))
        (:0
          (goto _label_3))
        (:1
          (Variables|Default|SetMaterial "/Engine/EngineMeshes/BackgroundMaterial.BackgroundMaterial"))
        (:2
          (Variables|Default|SetMaterial "/Engine/EngineMeshes/BackgroundMaterial.BackgroundMaterial"))))
    (:2
      ;[1 1 1] Метеорит
      (Variables|Default|SetMaterial "/Engine/MapTemplates/Materials/BasicAsset03.BasicAsset03")))
  (if (== (Utilities|Array|Length (Variables|Default|GetDynamicMats)) 0)
    (for (_array_element _array_index) (Rendering|Material|GetMaterials (Variables|Default|GetStaticMesh))
      (bind _returnvalue_3 (Rendering|Material|CreateDynamicMaterialInstance _array_element "None" :!class /Script/Engine.KismetMaterialLibrary))
      (Utilities|Array|Add (Variables|Default|GetDynamicMats) _returnvalue_3)
      (Rendering|Material|SetMaterial (Variables|Default|GetStaticMesh) _array_index _returnvalue_3)))
  (for (_ _array_index_2) (Variables|Default|GetDynamicMats)
    (Rendering|Material|SetMaterial (Variables|Default|GetStaticMesh) _array_index_2 (Variables|Default|GetMaterial))))

(event EventBeginPlay
  (CallFunction|SetStruct)
  (Utilities|Array|Clear (Variables|Default|GetDynamicMats)))

(fn ConstructionScript)

(fn GetStruct
  (return (Variables|Default|GetiIdStruct) (Variables|Default|GetbPassable)))