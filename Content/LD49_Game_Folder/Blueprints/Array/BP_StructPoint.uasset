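; BP_StructPoint is a grid point actor that holds a structure ID and shows the mesh for it.
; SetStruct stores the ID and switches on it to set the static mesh and a Passable flag, with only one snow field type passable and several IDs left meshless.
; BeginPlay starts each point at the empty, impassable ID, and GetStruct returns the ID and passability.
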(event Custom|SetStruct
  (params (iIndex :type Integer))
  (bind _staticmesh (Variables|Default|GetStaticMesh))
  (bind _output_get (Variables|Default|SetiIdStruct iIndex))
  (switch int _output_get
    (:0
      (Components|StaticMesh|SetStaticMesh _staticmesh 0)
      (Variables|Default|SetbPassable false))
    (:1
      (Components|StaticMesh|SetStaticMesh _staticmesh "/Game/LD49_Game_Folder/Meshes/Snow_Grid_Field_1.Snow_Grid_Field_1")
      (Variables|Default|SetbPassable true))
    (:2
      (Components|StaticMesh|SetStaticMesh _staticmesh "/Game/LD49_Game_Folder/Meshes/Snow_Grid_Field_1.Snow_Grid_Field_1")
      (Variables|Default|SetbPassable false))
    (:3
      (Components|StaticMesh|SetStaticMesh _staticmesh "/Game/LD49_Game_Folder/Assets/Cars/Cop_Cop.Cop_Cop")
      (Variables|Default|SetbPassable false))
    (:4
      (Components|StaticMesh|SetStaticMesh _staticmesh 0)
      (Variables|Default|SetbPassable false))
    (:5
      (Components|StaticMesh|SetStaticMesh _staticmesh 0)
      (Variables|Default|SetbPassable false))
    (:6
      (Components|StaticMesh|SetStaticMesh _staticmesh 0)
      (Variables|Default|SetbPassable false))
    (:7
      (Components|StaticMesh|SetStaticMesh _staticmesh 0)
      (Variables|Default|SetbPassable false))
    (:8
      (Components|StaticMesh|SetStaticMesh _staticmesh 0)
      (Variables|Default|SetbPassable false))
    (:9
      (Components|StaticMesh|SetStaticMesh _staticmesh 0)
      (Variables|Default|SetbPassable false))))

(event EventBeginPlay
  (CallFunction|SetStruct))

(fn ConstructionScript)

(fn GetStruct
  (return (Variables|Default|GetiIdStruct) (Variables|Default|GetbPassable)))