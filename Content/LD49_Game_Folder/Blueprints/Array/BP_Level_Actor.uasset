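; Level manager that builds a tile grid of field, danger and people actors, and runs group movement and timed hazards.
; BeginPlay seeds randomly sized red and blue teams, signed by colour.
; Move events step all groups by each one's angle, iteratively freezing blocked ones and dropping those leaving the field.
; Hazards target near groups, favouring off-centre ones, count down with animated warnings, then add damage or replace the tile.
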(event Custom|StartPositionPiople
  (Variables|Math|SetstructTemplytPioples (Variables|Math|GetstructRealPeoples))
  ;[1 1 1] Cleap Piople
  (for _array_element (Variables|Math|GetstructRealPeoples)
    (Default|SetPioples (.actorrefpiople (Utilities|GetPoint (.iX (Utilities|Struct|BreakSTRUCT_int_Point _array_element)) (.iY (Utilities|Struct|BreakSTRUCT_int_Point _array_element))))))
  ;[1 1 1] Create New Piople
  (Utilities|Array|Clear (Variables|Math|GetstructRealPeoples))
  (for _array_element_2 (Variables|Math|GetstructTemplytPioples)
    (if (not (Math|Boolean|ORBoolean (< (.iY (Utilities|Struct|BreakSTRUCT_int_Point _array_element_2)) 1) (== (.iY (Utilities|Struct|BreakSTRUCT_int_Point _array_element_2)) (Variables|OptionLevel|GetiFieldHeight)) (< (.iX (Utilities|Struct|BreakSTRUCT_int_Point _array_element_2)) 1) (== (.iX (Utilities|Struct|BreakSTRUCT_int_Point _array_element_2)) (Variables|OptionLevel|GetiFieldWidth))))
      (Default|SetPioples (.actorrefpiople (Utilities|GetPoint (.iX (Utilities|Struct|BreakSTRUCT_int_Point _array_element_2)) (.iY (Utilities|Struct|BreakSTRUCT_int_Point _array_element_2)))) (.iIndex (Utilities|Struct|BreakSTRUCT_int_Point _array_element_2)))
      (Utilities|Array|Add (Variables|Math|GetstructRealPeoples) _array_element_2))))

(event Custom|AddDamagePoint
  (params (iRaund :type Integer))
  (bind _structlistpredamage (Variables|Damage|GetstructListPreDamage))
  (Utilities|FlowControl|Sequence
    (:then_0
      (bind (_ix _iy) (CallFunction|GetTargetDamage))
      (Utilities|Array|Add _structlistpredamage (Utilities|Struct|MakeSTRUCT_int_Point _ix _iy 1 -2))
      (Default|SetAnimTextura (.actorrefstruct (Utilities|GetPoint _ix _iy)) 1 -2))
    (:then_1
      (if (< iRaund 15)
        (bind (_ix_2 _iy_2) (CallFunction|GetTargetDamage))
        (Utilities|Array|Add _structlistpredamage (Utilities|Struct|MakeSTRUCT_int_Point _ix_2 _iy_2 1 -2))
        (Default|SetAnimTextura (.actorrefstruct (Utilities|GetPoint _ix_2 _iy_2)) 1 -2)))
    (:then_2
      (if (< iRaund 10)
        (bind (_ix_3 _iy_3) (CallFunction|GetTargetDamage))
        (Utilities|Array|Add _structlistpredamage (Utilities|Struct|MakeSTRUCT_int_Point _ix_3 _iy_3 2 -3))
        (Default|SetAnimTextura (.actorrefstruct (Utilities|GetPoint _ix_3 _iy_3)) 2 -3)))
    (:then_3
      (if (< iRaund 5)
        (bind (_ix_4 _iy_4) (CallFunction|GetTargetDamage))
        (Utilities|Array|Add _structlistpredamage (Utilities|Struct|MakeSTRUCT_int_Point _ix_4 _iy_4 3 -1))
        (Default|SetAnimTextura (.actorrefstruct (Utilities|GetPoint _ix_4 _iy_4)) 3 -1)))))

(event Custom|eventMoveForvard
  (params (fForvard :type Float%20%28single-precision%29))
  (Variables|Default|SetfForward fForvard)
  (Variables|Default|SetfRight 0.0)
  (Utilities|Array|Clear (Variables|Default|GetiFreez))
  (for _index (range 0 5)
    (Utilities|Array|Clear (Variables|Math|GetstructTemplytPioples))
    (for (_array_element _array_index) (Variables|Math|GetstructRealPeoples)
      (if (== (Utilities|Array|FindItem (Variables|Default|GetiFreez) _array_index) -1)
        (bind _ianglemadify (Default|GetAngle (.actorrefpiople (Utilities|GetPoint (.iX (Utilities|Struct|BreakSTRUCT_int_Point _array_element)) (.iY (Utilities|Struct|BreakSTRUCT_int_Point _array_element))))))
        (|CollapseGraph_0 _ianglemadify
          (:OutputPin
            (bind _returnvalue (Utilities|Array|Add (Variables|Math|GetstructTemplytPioples) (Utilities|Struct|MakeSTRUCT_int_Point (+ (.iX (Utilities|Struct|BreakSTRUCT_int_Point _array_element)) (Math|Float|Truncate (Variables|Default|GetfRight))) (+ (.iY (Utilities|Struct|BreakSTRUCT_int_Point _array_element)) (Math|Float|Truncate (Variables|Default|GetfForward))) (.iIndex (Utilities|Struct|BreakSTRUCT_int_Point _array_element)))))
            (bind _bpassable (Default|GetStruct (.actorrefstruct (Utilities|GetPoint (+ (.iX (Utilities|Struct|BreakSTRUCT_int_Point _array_element)) (Math|Float|Truncate (Variables|Default|GetfRight))) (+ (.iY (Utilities|Struct|BreakSTRUCT_int_Point _array_element)) (Math|Float|Truncate (Variables|Default|GetfForward)))))))
            (for (_array_element_2 _array_index_2) (Variables|Math|GetstructTemplytPioples)
              (if (not (or _bpassable (Math|Boolean|ANDBoolean (== (.iX (Utilities|Struct|BreakSTRUCT_int_Point _array_element_2)) (+ (.iX (Utilities|Struct|BreakSTRUCT_int_Point _array_element)) (Math|Float|Truncate (Variables|Default|GetfRight)))) (== (.iY (Utilities|Struct|BreakSTRUCT_int_Point _array_element_2)) (+ (.iY (Utilities|Struct|BreakSTRUCT_int_Point _array_element)) (Math|Float|Truncate (Variables|Default|GetfForward)))) (!= _returnvalue _array_index_2) true)))
                (Utilities|Array|Add (Variables|Default|GetiFreez) _array_index)))))
        (else
          (Utilities|Array|Add (Variables|Math|GetstructTemplytPioples) (Utilities|Struct|MakeSTRUCT_int_Point (.iX (Utilities|Struct|BreakSTRUCT_int_Point _array_element)) (.iY (Utilities|Struct|BreakSTRUCT_int_Point _array_element)) (.iIndex (Utilities|Struct|BreakSTRUCT_int_Point _array_element))))))))
  ;[1 1 1] Cleap Piople
  (for _array_element_3 (Variables|Math|GetstructRealPeoples)
    (Default|SetPioples (.actorrefpiople (Utilities|GetPoint (.iX (Utilities|Struct|BreakSTRUCT_int_Point _array_element_3)) (.iY (Utilities|Struct|BreakSTRUCT_int_Point _array_element_3))))))
  ;[1 1 1] Create New Piople
  (Utilities|Array|Clear (Variables|Math|GetstructRealPeoples))
  (for _array_element_4 (Variables|Math|GetstructTemplytPioples)
    (if (not (Math|Boolean|ORBoolean (< (.iY (Utilities|Struct|BreakSTRUCT_int_Point _array_element_4)) 1) (== (.iY (Utilities|Struct|BreakSTRUCT_int_Point _array_element_4)) (Variables|OptionLevel|GetiFieldHeight)) (< (.iX (Utilities|Struct|BreakSTRUCT_int_Point _array_element_4)) 1) (== (.iX (Utilities|Struct|BreakSTRUCT_int_Point _array_element_4)) (Variables|OptionLevel|GetiFieldWidth))))
      (Default|SetPioples (.actorrefpiople (Utilities|GetPoint (.iX (Utilities|Struct|BreakSTRUCT_int_Point _array_element_4)) (.iY (Utilities|Struct|BreakSTRUCT_int_Point _array_element_4)))) (.iIndex (Utilities|Struct|BreakSTRUCT_int_Point _array_element_4)))
      (Utilities|Array|Add (Variables|Math|GetstructRealPeoples) _array_element_4))))

(event Custom|eventMoveRight
  (params (fRight :type Float%20%28single-precision%29))
  (Variables|Default|SetfRight fRight)
  (Variables|Default|SetfForward 0.0)
  (Utilities|Array|Clear (Variables|Default|GetiFreez))
  (for _index (range 0 5)
    (Utilities|Array|Clear (Variables|Math|GetstructTemplytPioples))
    (for (_array_element _array_index) (Variables|Math|GetstructRealPeoples)
      (if (== (Utilities|Array|FindItem (Variables|Default|GetiFreez) _array_index) -1)
        (bind _ianglemadify (Default|GetAngle (.actorrefpiople (Utilities|GetPoint (.iX (Utilities|Struct|BreakSTRUCT_int_Point _array_element)) (.iY (Utilities|Struct|BreakSTRUCT_int_Point _array_element))))))
        (|CollapseGraph_0 _ianglemadify
          (:OutputPin
            (bind _returnvalue (Utilities|Array|Add (Variables|Math|GetstructTemplytPioples) (Utilities|Struct|MakeSTRUCT_int_Point (+ (.iX (Utilities|Struct|BreakSTRUCT_int_Point _array_element)) (Math|Float|Truncate (Variables|Default|GetfRight))) (+ (.iY (Utilities|Struct|BreakSTRUCT_int_Point _array_element)) (Math|Float|Truncate (Variables|Default|GetfForward))) (.iIndex (Utilities|Struct|BreakSTRUCT_int_Point _array_element)))))
            (bind _bpassable (Default|GetStruct (.actorrefstruct (Utilities|GetPoint (+ (.iX (Utilities|Struct|BreakSTRUCT_int_Point _array_element)) (Math|Float|Truncate (Variables|Default|GetfRight))) (+ (.iY (Utilities|Struct|BreakSTRUCT_int_Point _array_element)) (Math|Float|Truncate (Variables|Default|GetfForward)))))))
            (for (_array_element_2 _array_index_2) (Variables|Math|GetstructTemplytPioples)
              (if (not (or _bpassable (Math|Boolean|ANDBoolean (== (.iX (Utilities|Struct|BreakSTRUCT_int_Point _array_element_2)) (+ (.iX (Utilities|Struct|BreakSTRUCT_int_Point _array_element)) (Math|Float|Truncate (Variables|Default|GetfRight)))) (== (.iY (Utilities|Struct|BreakSTRUCT_int_Point _array_element_2)) (+ (.iY (Utilities|Struct|BreakSTRUCT_int_Point _array_element)) (Math|Float|Truncate (Variables|Default|GetfForward)))) (!= _returnvalue _array_index_2) true)))
                (Utilities|Array|Add (Variables|Default|GetiFreez) _array_index)))))
        (else
          (Utilities|Array|Add (Variables|Math|GetstructTemplytPioples) (Utilities|Struct|MakeSTRUCT_int_Point (.iX (Utilities|Struct|BreakSTRUCT_int_Point _array_element)) (.iY (Utilities|Struct|BreakSTRUCT_int_Point _array_element)) (.iIndex (Utilities|Struct|BreakSTRUCT_int_Point _array_element))))))))
  ;[1 1 1] Cleap Piople
  (for _array_element_3 (Variables|Math|GetstructRealPeoples)
    (Default|SetPioples (.actorrefpiople (Utilities|GetPoint (.iX (Utilities|Struct|BreakSTRUCT_int_Point _array_element_3)) (.iY (Utilities|Struct|BreakSTRUCT_int_Point _array_element_3))))))
  ;[1 1 1] Create New Piople
  (Utilities|Array|Clear (Variables|Math|GetstructRealPeoples))
  (for _array_element_4 (Variables|Math|GetstructTemplytPioples)
    (if (not (Math|Boolean|ORBoolean (< (.iY (Utilities|Struct|BreakSTRUCT_int_Point _array_element_4)) 1) (== (.iY (Utilities|Struct|BreakSTRUCT_int_Point _array_element_4)) (Variables|OptionLevel|GetiFieldHeight)) (< (.iX (Utilities|Struct|BreakSTRUCT_int_Point _array_element_4)) 1) (== (.iX (Utilities|Struct|BreakSTRUCT_int_Point _array_element_4)) (Variables|OptionLevel|GetiFieldWidth))))
      (Default|SetPioples (.actorrefpiople (Utilities|GetPoint (.iX (Utilities|Struct|BreakSTRUCT_int_Point _array_element_4)) (.iY (Utilities|Struct|BreakSTRUCT_int_Point _array_element_4)))) (.iIndex (Utilities|Struct|BreakSTRUCT_int_Point _array_element_4)))
      (Utilities|Array|Add (Variables|Math|GetstructRealPeoples) _array_element_4))))

(event Custom|TikeDamage
  (Utilities|Array|Clear (Variables|Damage|GetstructListPreDamageTemplate))
  (for _array_element (Variables|Damage|GetstructListPreDamage)
    (bind _returnvalue (Utilities|Array|Add (Variables|Damage|GetstructListPreDamageTemplate) (Utilities|Struct|MakeSTRUCT_int_Point (.iX (Utilities|Struct|BreakSTRUCT_int_Point _array_element)) (.iY (Utilities|Struct|BreakSTRUCT_int_Point _array_element)) (.iIndex (Utilities|Struct|BreakSTRUCT_int_Point _array_element)) (+ (.iTike (Utilities|Struct|BreakSTRUCT_int_Point _array_element)) 1))))
    (if (>= (+ (.iTike (Utilities|Struct|BreakSTRUCT_int_Point _array_element)) 1) 0)
      (Utilities|Array|RemoveIndex (Variables|Damage|GetstructListPreDamageTemplate) _returnvalue)
      (if (== (.iIndex (Utilities|Struct|BreakSTRUCT_int_Point _array_element)) 3)
        (Default|SetStruct (.actorrefstruct (Utilities|GetPoint (.iX (Utilities|Struct|BreakSTRUCT_int_Point _array_element)) (.iY (Utilities|Struct|BreakSTRUCT_int_Point _array_element)))))
        (else
          (Default|AddPoinDamage (.actorrefdanger (Utilities|GetPoint (.iX (Utilities|Struct|BreakSTRUCT_int_Point _array_element)) (.iY (Utilities|Struct|BreakSTRUCT_int_Point _array_element)))) (.iIndex (Utilities|Struct|BreakSTRUCT_int_Point _array_element)))))
      (else
        (Default|SetAnimTextura (.actorrefstruct (Utilities|GetPoint (.iX (Utilities|Struct|BreakSTRUCT_int_Point _array_element)) (.iY (Utilities|Struct|BreakSTRUCT_int_Point _array_element)))) (.iIndex (Utilities|Struct|BreakSTRUCT_int_Point _array_element)) (.iTike (Utilities|Struct|BreakSTRUCT_int_Point _array_element))))))
  (Variables|Damage|SetstructListPreDamage (Variables|Damage|GetstructListPreDamageTemplate)))

(event EventBeginPlay
  (bind _structpiopleclocation (Variables|OptionLevel|GetstructPioplecLocation))
  (bind _structpiopleclocation_2 (Variables|OptionLevel|GetstructPioplecLocation))
  (bind _structpiopleclocation_3 (Variables|OptionLevel|GetstructPioplecLocation))
  (bind _structpiopleclocation_4 (Variables|OptionLevel|GetstructPioplecLocation))
  (bind _returnvalue (Utilities|Array|Length _structpiopleclocation))
  (bind _returnvalue_2 (Utilities|Array|Length _structpiopleclocation_3))
  (bind _returnvalue_3 (Math|Random|RandomInteger _returnvalue_2))
  (bind _returnvalue_4 (Math|Random|RandomInteger _returnvalue))
  (bind _output (Utilities|Array|Get(acopy) _structpiopleclocation_2 _returnvalue_4))
  (bind _output_2 (Utilities|Array|Get(acopy) _structpiopleclocation_4 _returnvalue_3))
  ;[1 0.6618 0.4892] Generation Date Level
  (for _index (range 0 (Variables|OptionLevel|GetiFieldHeight))
    (Utilities|Array|Clear (Utilities|Struct|BreakSTRUCT_Line_Array (Variables|Math|GetstructLineLevel)))
    (for _index_2 (range 0 (Variables|OptionLevel|GetiFieldWidth))
      (|CreateBP _index _index_2)
      (Default|SetStruct (Variables|2DArray|GetrefStruct) 1)
      (for _array_element (Variables|OptionLevel|GetstructPositionObject)
        (if (Math|Boolean|ANDBoolean (== _index (.iY (Utilities|Struct|BreakSTRUCT_int_Point _array_element))) (== (.iX (Utilities|Struct|BreakSTRUCT_int_Point _array_element)) _index_2) true)
          (Default|SetStruct (Variables|2DArray|GetrefStruct) (.iIndex (Utilities|Struct|BreakSTRUCT_int_Point _array_element)))))
      (Variables|Math|SetstructPointLevel (Utilities|Struct|MakeSTRUCT_Point_Array (Variables|2DArray|GetrefStruct) (Variables|2DArray|GetrefDanger) (Variables|2DArray|GetrefPiople)))
      (Utilities|Array|Add (Utilities|Struct|BreakSTRUCT_Line_Array (Variables|Math|GetstructLineLevel)) (Variables|Math|GetstructPointLevel)))
    (Utilities|Array|Add (Utilities|Struct|BreakSTRUCT_2D_Array (Variables|Math|Getstruct2DArrayLevel)) (Variables|Math|GetstructLineLevel)))
  (Utilities|Array|Clear (Variables|Math|GetstructRealPeoples))
  ;[1 0.5069 0.4671] Red Piople
  (for _index_3 (range 0 4)
    (if (and (> (Variables|OptionLevel|GetiMaxPiopleInRed) 0) (> (Utilities|Array|Length (Variables|OptionLevel|GetstructPioplecLocation)) 0))
      (bind _output_get (Variables|Default|SetiRndPiopleInTeam (Math|Random|RandomIntegerinRange 1 9)))
      (if (<= _output_get (Variables|OptionLevel|GetiMaxPiopleInRed))
        _
        (else
          (Variables|Default|SetiRndPiopleInTeam (Variables|OptionLevel|GetiMaxPiopleInRed))))
      (Variables|OptionLevel|SetiMaxPiopleInRed (- (Variables|OptionLevel|GetiMaxPiopleInRed) (Variables|Default|GetiRndPiopleInTeam)))
      (Utilities|Array|Add (Variables|Math|GetstructRealPeoples) (Utilities|Struct|MakeSTRUCT_int_Point (.ix _output_2) (.iy _output_2) (Variables|Default|GetiRndPiopleInTeam)))
      (Utilities|Array|RemoveIndex (Variables|OptionLevel|GetstructPioplecLocation) _returnvalue_3)))
  ;[0.3197 0.7122 1] Blue Piople
  (for _index_4 (range 0 4)
    (if (and (> (Variables|OptionLevel|GetiMaxPiopleInBlue) 0) (> (Utilities|Array|Length (Variables|OptionLevel|GetstructPioplecLocation)) 0))
      (bind _output_get_2 (Variables|Default|SetiRndPiopleInTeam (Math|Random|RandomIntegerinRange 1 9)))
      (if (<= _output_get_2 (Variables|OptionLevel|GetiMaxPiopleInBlue))
        _
        (else
          (Variables|Default|SetiRndPiopleInTeam (Variables|OptionLevel|GetiMaxPiopleInBlue))))
      (Variables|OptionLevel|SetiMaxPiopleInBlue (- (Variables|OptionLevel|GetiMaxPiopleInBlue) (Variables|Default|GetiRndPiopleInTeam)))
      (Utilities|Array|Add (Variables|Math|GetstructRealPeoples) (Utilities|Struct|MakeSTRUCT_int_Point (.ix _output) (.iy _output) (* (Variables|Default|GetiRndPiopleInTeam) -1)))
      (Utilities|Array|RemoveIndex (Variables|OptionLevel|GetstructPioplecLocation) _returnvalue_4)))
  (CallFunction|StartPositionPiople))

(fn ConstructionScript)

(fn GetTargetDamage
  (bind _structrealpeoples (Variables|Math|GetstructRealPeoples))
  (for (_array_element _array_index) _structrealpeoples
    (if (Math|Boolean|ANDBoolean (== (LocalVariables|GetiTotalPoint) -1) (< (Math|Random|RandomIntegerinRange 0 100) (+ (* (+ (Math|Integer|Absolute(Integer) (- (.iX (Utilities|Struct|BreakSTRUCT_int_Point _array_element)) (/ (Variables|OptionLevel|GetiFieldWidth) 2))) (Math|Integer|Absolute(Integer) (- (.iY (Utilities|Struct|BreakSTRUCT_int_Point _array_element)) (/ (Variables|OptionLevel|GetiFieldHeight) 2)))) 8) (.iIndex (Utilities|Struct|BreakSTRUCT_int_Point _array_element)))) true)
      (LocalVariables|SetiTotalPoint _array_index)))
  (if (> (LocalVariables|GetiTotalPoint) -1)
    (return (+ (.ix (Utilities|Array|Get(acopy) _structrealpeoples (LocalVariables|GetiTotalPoint))) (Math|Random|RandomIntegerinRange -1 1)) (+ (.iy (Utilities|Array|Get(acopy) _structrealpeoples (LocalVariables|GetiTotalPoint))) (Math|Random|RandomIntegerinRange -1 1)))))