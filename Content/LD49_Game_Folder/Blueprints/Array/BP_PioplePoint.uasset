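; BP_PioplePoint is an actor that displays a people count through a widget component.
; It starts hidden; SetPioples hides it when the count is zero, otherwise writes the number into its BP_Widget_Piople widget and shows the root and its children.
; It also stores an angle modifier, exposed through simple GetAngle and SetAngle functions, which this Blueprint does not otherwise use.
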(event EventBeginPlay
  (Rendering|SetVisibility (Variables|Default|GetDefaultSceneRoot) false true))

(event Collision|EventActorBeginOverlap
  (params (OtherActor :type Actor%20Object%20Reference)))

(event EventTick
  (params (DeltaSeconds :type Float%20%28single-precision%29)))

(fn ConstructionScript)

(fn SetPioples
  (params (iNumber :type Integer))
  (bind _output_get (Variables|Default|SetiNumber iNumber))
  (if (!= _output_get 0)
    (bind _asbp_widget_piople (Utilities|Casting|CastToBP_Widget_Piople (UserInterface|GetUserWidgetObject (Variables|Default|GetWidget))))
    (Default|SetTextInfo _asbp_widget_piople (Utilities|Text|ToText(Integer) _output_get))
    (Rendering|SetVisibility (Variables|Default|GetDefaultSceneRoot) true true)
    (else
      (Rendering|SetVisibility (Variables|Default|GetDefaultSceneRoot) false true))))

(fn GetAngle
  (return (Variables|Default|GetiAngleMadify)))

(fn SetAngle
  (params (iAngleMadify :type Integer))
  (Variables|Default|SetiAngleMadify iAngleMadify)
  (return))