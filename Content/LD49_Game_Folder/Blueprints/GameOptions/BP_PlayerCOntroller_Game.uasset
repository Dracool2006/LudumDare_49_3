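; Player controller for the game mode that turns WASD presses into discrete, turn-based moves on a level actor.
; On BeginPlay it spawns BP_Level_Actor, shows BP_Widget_Game with the round counter and plays the game sound cue.
; Each press moves via the level actor, decrements the counter, updates the widget, then ticks danger regions and damage.
; A shared Press flag blocks further moves until a movement key is released.
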(event EventBeginPlay
  (bind _returnvalue (Game|SpawnActorfromClass "/Game/LD49_Game_Folder/Blueprints/Array/BP_Level_Actor.BP_Level_Actor_C" (Math|Transform|MakeTransform "0, 0, 0") "Undefined" 0 0))
  (Variables|Default|SetrefActor _returnvalue)
  (bind _returnvalue_2 (UserInterface|CreateWidget "/Game/LD49_Game_Folder/Blueprints/UMG/BP_Widget_Game.BP_Widget_Game_C"))
  (bind _output_get (Variables|Default|SetrefWidget _returnvalue_2))
  (UserInterface|Viewport|AddtoViewport _output_get 0)
  (Audio|PlaySound2D "/Game/LD49_Game_Folder/Sound/Gameplay/CUE_Game.CUE_Game" 1.0 1.0 0.0 0 0)
  (Default|SetRaund (Variables|Default|GetrefWidget) (Utilities|Text|ToText(Integer) (Variables|Default|GetiGlobalTimer))))

(event Input|KeyboardEvents|A
  (params (Key :type Key%20Structure :default "None"))
  (bind _refactor (Variables|Default|GetrefActor))
  (:Pressed
    (if (not (Variables|Default|GetbPress))
      (Variables|Default|SetbPress true)
      (Default|EventMoveForvard (Variables|Default|GetrefActor) -1.0)
      (bind _output_get (Variables|Default|SetiGlobalTimer (- (Variables|Default|GetiGlobalTimer) 1)))
      (Default|SetRaund (Variables|Default|GetrefWidget) (Utilities|Text|ToText(Integer) _output_get))
      (Default|EventDangetRegionTick _refactor)
      (Default|TikeDamage _refactor)
      (Default|AddDamagePoint _refactor (Variables|Default|GetiGlobalTimer))))
  (:Released
    (Variables|Default|SetbPress false)))

(event Input|KeyboardEvents|D
  (params (Key :type Key%20Structure :default "None"))
  (bind _refactor (Variables|Default|GetrefActor))
  (:Pressed
    (if (not (Variables|Default|GetbPress))
      (Variables|Default|SetbPress true)
      (Default|EventMoveForvard (Variables|Default|GetrefActor) 1.0)
      (bind _output_get (Variables|Default|SetiGlobalTimer (- (Variables|Default|GetiGlobalTimer) 1)))
      (Default|SetRaund (Variables|Default|GetrefWidget) (Utilities|Text|ToText(Integer) _output_get))
      (Default|EventDangetRegionTick _refactor)
      (Default|TikeDamage _refactor)
      (Default|AddDamagePoint _refactor (Variables|Default|GetiGlobalTimer))))
  (:Released
    (Variables|Default|SetbPress false)))

(event Input|KeyboardEvents|W
  (params (Key :type Key%20Structure :default "None"))
  (bind _refactor (Variables|Default|GetrefActor))
  (:Pressed
    (if (not (Variables|Default|GetbPress))
      (Variables|Default|SetbPress true)
      (Default|EventMoveRight (Variables|Default|GetrefActor) 1.0)
      (bind _output_get (Variables|Default|SetiGlobalTimer (- (Variables|Default|GetiGlobalTimer) 1)))
      (Default|SetRaund (Variables|Default|GetrefWidget) (Utilities|Text|ToText(Integer) _output_get))
      (Default|EventDangetRegionTick _refactor)
      (Default|TikeDamage _refactor)
      (Default|AddDamagePoint _refactor (Variables|Default|GetiGlobalTimer))))
  (:Released
    (Variables|Default|SetbPress false)))

(event Input|KeyboardEvents|S
  (params (Key :type Key%20Structure :default "None"))
  (bind _refactor (Variables|Default|GetrefActor))
  (:Pressed
    (if (not (Variables|Default|GetbPress))
      (Variables|Default|SetbPress true)
      (Default|EventMoveRight (Variables|Default|GetrefActor) -1.0)
      (bind _output_get (Variables|Default|SetiGlobalTimer (- (Variables|Default|GetiGlobalTimer) 1)))
      (Default|SetRaund (Variables|Default|GetrefWidget) (Utilities|Text|ToText(Integer) _output_get))
      (Default|EventDangetRegionTick _refactor)
      (Default|TikeDamage _refactor)
      (Default|AddDamagePoint _refactor (Variables|Default|GetiGlobalTimer))))
  (:Released
    (Variables|Default|SetbPress false)))

(fn ConstructionScript)